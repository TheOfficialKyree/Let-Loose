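; BP_Save is a save point actor that writes to the "save1" slot when BP_JamesLevel1 hits its box.
; On BeginPlay it either loads BP_SaveGame and moves itself to the stored PlayerPos, or creates a save holding its own transform.
; A hit stores the actor's own transform, not the player's, but first checks an empty slot name rather than "save1", and only the load branch caches the save object.
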(event OnComponentHit(Box)
  (params (HitComponent :type Primitive%20Component%20Object%20Reference) (OtherActor :type Actor%20Object%20Reference) (OtherComp :type Primitive%20Component%20Object%20Reference) (NormalImpulse :type Vector :default "0, 0, 0") (Hit :type Hit%20Result%20Structure%20%28by%20ref%29))
  (bind _as_bp_save_game (Variables|Default|GetAs%20BP%20Save%20Game))
  (Utilities|Casting|CastToBP_JamesLevel1 OtherActor)
  (bind _returnvalue (SaveGame|DoesSaveGameExist))
  (if _returnvalue
    (Variables|/Game/LetLoose/Levels/BP_SaveGame.BP_SaveGame_C|SetplayerPos _as_bp_save_game (Transformation|GetActorTransform))
    (SaveGame|SaveGametoSlot _as_bp_save_game "save1")
    (Development|PrintString "GAME SAVED")))

(event EventBeginPlay
  (bind _returnvalue (SaveGame|DoesSaveGameExist "save1"))
  (if _returnvalue
    (bind _returnvalue_2 (SaveGame|LoadGamefromSlot "save1"))
    (bind _asbp_save_game (Utilities|Casting|CastToBP_SaveGame _returnvalue_2))
    (Variables|Default|SetAs%20BP%20Save%20Game _asbp_save_game)
    (Transformation|SetActorTransform (Variables|/Game/LetLoose/Levels/BP_SaveGame.BP_SaveGame_C|GetplayerPos _asbp_save_game))
    (else
      (bind _returnvalue_3 (SaveGame|CreateSaveGameObject "/Game/LetLoose/Levels/BP_SaveGame.BP_SaveGame_C"))
      (Variables|/Game/LetLoose/Levels/BP_SaveGame.BP_SaveGame_C|SetplayerPos _returnvalue_3 (Transformation|GetActorTransform))
      (SaveGame|SaveGametoSlot _returnvalue_3 "save1"))))

(event Collision|EventActorBeginOverlap
  (params (OtherActor :type Actor%20Object%20Reference)))

(event EventTick
  (params (DeltaSeconds :type Float%20%28single-precision%29)))

(fn ConstructionScript)